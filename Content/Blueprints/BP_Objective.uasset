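; BP_Objective is the level goal that lets the player win on overlap once they have enough trailers.
; On BeginPlay it writes the required trailer count into the FinishText user widget of its Widget component.
; On overlap it compares BP_PlayerCharacter's Trailers array with RequiredTrailers.
; Success shows WinScreen once and calls StopHoldingButtons on the player, while a shortfall prints the missing count and adds a new W_NeedMoreTrailers widget each time.
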(event EventBeginPlay
  (bind _asfinish_text (Utilities|Casting|CastToFinishText (UserInterface|GetUserWidgetObject (Variables|Default|GetWidget))))
  (Rendering|Components|TextRender|SetText (Variables|/Game/Widgets/FinishText.FinishText_C|GetTrailersRequired _asfinish_text) (Utilities|Text|FormatText "Trailers Required: {Number}" (Variables|Default|GetRequiredTrailers))))

(event Collision|EventActorBeginOverlap
  (params (OtherActor :type Actor%20Object%20Reference))
  (bind _asbp_player_character (Utilities|Casting|CastToBP_PlayerCharacter OtherActor))
  (if (>= (Utilities|Array|Length (Variables|/Game/Blueprints/BP_PlayerCharacter.BP_PlayerCharacter_C|GetTrailers _asbp_player_character)) (Variables|Default|GetRequiredTrailers))
    (Utilities|FlowControl|DoOnce false
      (:Completed
        (Development|PrintString "You win!")
        (bind _returnvalue (UserInterface|CreateWidget "/Game/Widgets/WinScreen.WinScreen_C" (Game|GetPlayerController 0)))
        (UserInterface|Viewport|AddtoViewport _returnvalue 0)
        (Default|StopHoldingButtons _asbp_player_character)))
    (else
      (Development|PrintString (Utilities|String|Append "You require " (Utilities|String|ToString(Integer) (- (Variables|Default|GetRequiredTrailers) (Utilities|Array|Length (Variables|/Game/Blueprints/BP_PlayerCharacter.BP_PlayerCharacter_C|GetTrailers _asbp_player_character)))) " more trailer(s) to progress"))
      (bind _returnvalue_2 (UserInterface|CreateWidget "/Game/Widgets/W_NeedMoreTrailers.W_NeedMoreTrailers_C" (Game|GetPlayerController 0)))
      (UserInterface|Viewport|AddtoViewport _returnvalue_2 0))))

(fn ConstructionScript)