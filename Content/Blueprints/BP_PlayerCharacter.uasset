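; BP_PlayerCharacter is a physics-driven player pawn that moves by the recoil of its two guns.
; Holding LeftFire or RightFire repeatedly spawns BP_PlayerProjectile from that side's fire point and impulses the capsule backward, using DoOnce, a short delay and self-calling events.
; Tick applies opposite yaw torque for each held side, none when both are held.
; Reverse uses the same loop to impulse the capsule forward without firing.
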(event Custom|ReverseOut
  ;[1 1 1] Movement/Shooting
  (Utilities|FlowControl|DoOnce false :!label _label
    (:Completed
      (Physics|AddImpulse (Variables|Collision|GetCapsuleComponent) (* (Transformation|GetActorForwardVector) 4e+03) "None" false)
      (Utilities|FlowControl|Delay 0.05)
      (Utilities|FlowControl|Sequence
        (:then_0
          (goto _label Reset))
        (:then_1
          (if (Variables|Default|GetReverseHeld)
            (CallFunction|ReverseOut)))))))

(event Custom|ShootLeft
  ;[1 1 1] Movement/Shooting
  (Utilities|FlowControl|DoOnce false :!label _label
    (:Completed
      (Physics|AddImpulse (Variables|Collision|GetCapsuleComponent) (* (Transformation|GetActorForwardVector) -5e+03) "None" false)
      (CallFunction|ShootProjectile (Variables|Default|GetFirepoint1))
      (Utilities|FlowControl|Delay 0.05)
      (Utilities|FlowControl|Sequence
        (:then_0
          (goto _label Reset))
        (:then_1
          (if (Variables|Default|GetLeftHeld)
            (CallFunction|ShootLeft)))))))

(event Custom|ShootRight
  ;[1 1 1] Movement/Shooting
  (Utilities|FlowControl|DoOnce false :!label _label
    (:Completed
      (Physics|AddImpulse (Variables|Collision|GetCapsuleComponent) (* (Transformation|GetActorForwardVector) -5e+03) "None" false)
      (CallFunction|ShootProjectile (Variables|Default|GetFirepoint2))
      (Utilities|FlowControl|Delay 0.05)
      (Utilities|FlowControl|Sequence
        (:then_0
          (goto _label Reset))
        (:then_1
          (if (Variables|Default|GetRightHeld)
            (CallFunction|ShootRight)))))))

(event EventTick
  (params (DeltaSeconds :type Float%20%28single-precision%29))
  (if (and (Variables|Default|GetLeftHeld) (Variables|Default|GetRightHeld))
    (Class|PrimitiveComponent|AddTorqueinDegrees (Variables|Collision|GetCapsuleComponent) "0, 0, 0" "None" true)
    (else
      (Utilities|FlowControl|Sequence
        (:then_0
          (if (Variables|Default|GetLeftHeld)
            (Class|PrimitiveComponent|AddTorqueinDegrees (Variables|Collision|GetCapsuleComponent) "0, 0,-60.000000" "None" true)))
        (:then_1
          (if (Variables|Default|GetRightHeld)
            (Class|PrimitiveComponent|AddTorqueinDegrees (Variables|Collision|GetCapsuleComponent) "0, 0,60.000000" "None" true)))))))

(event Input|ActionEvents|InputActionLeftFire
  (params (Key :type Key%20Structure :default "None"))
  ;[1 1 1] Movement/Shooting
  (:Pressed
    (Variables|Default|SetLeftHeld true)
    (CallFunction|ShootLeft))
  (:Released
    (Variables|Default|SetLeftHeld false)))

(event Input|ActionEvents|InputActionRightFire
  (params (Key :type Key%20Structure :default "None"))
  ;[1 1 1] Movement/Shooting
  (:Pressed
    (Variables|Default|SetRightHeld true)
    (CallFunction|ShootRight))
  (:Released
    (Variables|Default|SetRightHeld false)))

(event Input|ActionEvents|InputActionReverse
  (params (Key :type Key%20Structure :default "None"))
  ;[1 1 1] Movement/Shooting
  (:Pressed
    (Variables|Default|SetReverseHeld true)
    (CallFunction|ReverseOut)
    (Class|PrimitiveComponent|SetAngularDamping (Variables|Collision|GetCapsuleComponent) 0.5))
  (:Released
    (Variables|Default|SetReverseHeld false)
    (Class|PrimitiveComponent|SetAngularDamping (Variables|Collision|GetCapsuleComponent) 0.5)))

(fn ConstructionScript)

(fn ShootProjectile
  (params (FirePoint :type Scene%20Component%20Object%20Reference))
  (bind _returnvalue (Transformation|GetWorldTransform FirePoint))
  (Game|SpawnActorfromClass "/Game/Blueprints/BP_PlayerProjectile.BP_PlayerProjectile_C" (Math|Transform|MakeTransform (.location _returnvalue) (.rotation _returnvalue) "1,1,1") "Undefined" 0 0))