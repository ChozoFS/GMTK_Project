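; BP_Trailer is a trailer actor that attaches to BP_PlayerCharacter on overlap.
; On overlap it joins the character's Trailers array, attaches to its TrailerAttach component and takes a relative offset scaled by its index, forming a chain.
; It then calls RecoverTrailer on the player 0 character.
; SpreadOut moves it by a random X and Y offset and adds its current Z again, doubling its height.
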(event Custom|Spread%20Out
  (Variables|Default|SetInitialLocation (Transformation|GetActorLocation))
  (Transformation|SetActorLocation (+ (Variables|Default|GetInitialLocation) (Math|Vector|MakeVector (Math|Random|RandomFloatinRange -8e+02 8e+02) (Math|Random|RandomFloatinRange -8e+02 8e+02) (.Z (Math|Vector|BreakVector (Variables|Default|GetInitialLocation))))) false false))

(event Collision|EventActorBeginOverlap
  (params (OtherActor :type Actor%20Object%20Reference))
  (bind _asbp_player_character (Utilities|Casting|CastToBP_PlayerCharacter OtherActor))
  (Development|PrintString "This Will Attach to the Player Character")
  (Utilities|Array|Add (Variables|/Game/Blueprints/BP_PlayerCharacter.BP_PlayerCharacter_C|GetTrailers _asbp_player_character) self)
  (Transformation|AttachComponentToComponent (Variables|/Game/Blueprints/BP_PlayerCharacter.BP_PlayerCharacter_C|GetTrailerAttach _asbp_player_character) "None" "SnapToTarget" "KeepRelative" "KeepRelative" false)
  (Transformation|SetActorRelativeLocation (* (- (Variables|/Script/Engine.SceneComponent|GetRelativeLocation (Variables|/Game/Blueprints/BP_PlayerCharacter.BP_PlayerCharacter_C|GetTrailerAttach _asbp_player_character)) (Math|Vector|MakeVector (Variables|Default|GetXOffset) 0.0 0.0)) (Math|Conversions|ToFloat(Integer) (- (Utilities|Array|Length (Variables|/Game/Blueprints/BP_PlayerCharacter.BP_PlayerCharacter_C|GetTrailers _asbp_player_character)) 1))))
  (bind _asbp_player_character_2 (Utilities|Casting|CastToBP_PlayerCharacter (Game|GetPlayerCharacter 0)))
  (Default|RecoverTrailer _asbp_player_character_2))

(fn ConstructionScript)