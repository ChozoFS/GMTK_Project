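; BP_WorldMessage is a world message Blueprint that displays configurable text through a widget.
; On BeginPlay it hides the widget, writes its Text variable into the WorldMessageWidget's text block, then reveals it after a five-second delay.
; The MakeVisible event jumps straight to the reveal step, showing the widget without waiting for the delay.
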(event Custom|MakeVisible
  (Rendering|SetVisibility (Variables|Default|GetWidget) true false))

(event EventBeginPlay
  (Rendering|SetVisibility (Variables|Default|GetWidget) false false)
  (bind _asworld_message_widget (Utilities|Casting|CastToWorldMessageWidget (UserInterface|GetUserWidgetObject (Variables|Default|GetWidget))))
  (Rendering|Components|TextRender|SetText (Variables|/Game/Widgets/WorldMessageWidget.WorldMessageWidget_C|GetTextBlock_0 _asworld_message_widget) (Variables|Default|GetText))
  (Utilities|FlowControl|Delay 5.0)
  (Rendering|SetVisibility (Variables|Default|GetWidget) true false))

(fn ConstructionScript)