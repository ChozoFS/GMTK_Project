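; First-person shooter player projectile actor that launches a physics sphere and cleans itself up.
; On BeginPlay it sets the sphere's linear velocity along the root's forward vector, scaled from BulletSpeed.
; Tick counts down DestroyDelay, then destroys the actor once it has not been rendered recently, so visible bullets persist.
; It contains no hit, damage or overlap logic.
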(event EventBeginPlay
  (Physics|SetPhysicsLinearVelocity (Variables|Default|GetSphere1) (* (* (Math|Vector|GetForwardVector (Variables|Default|GetDefaultSceneRoot)) (Variables|Default|GetBulletSpeed)) 1e+02) false "None"))

(event Collision|EventActorBeginOverlap
  (params (OtherActor :type Actor%20Object%20Reference)))

(event EventTick
  (params (DeltaSeconds :type Float%20%28single-precision%29))
  (bind _output_get (Variables|Default|SetDestroyDelay (- (Variables|Default|GetDestroyDelay) DeltaSeconds)))
  (if (<= _output_get 0.0)
    ;[0.556 0.5008 1] If bullet goes off screen, destroy it
    (if (not (Class|Actor|WasRecentlyRendered 0.5))
      (Actor|DestroyActor))))

(fn ConstructionScript)