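; BP_EnemyBase is an FPS enemy that chases the player and fires projectiles at random intervals.
; Every tick it moves toward the player character with SimpleMoveToActor and counts down a timer, spawning an EnemyProjectile_FPS just ahead of itself and re-randomizing the delay.
; Overlapping a player projectile destroys both the projectile and the enemy.
; An AIMoveTo node is left unconnected.
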(event EventBeginPlay
  ;[1 1 1] Shoot Projectile After Random Time Has Passed
  (Variables|Default|SetShootTimer (Math|Random|RandomFloatinRange 0.5 2.0)))

(event Collision|EventActorBeginOverlap
  (params (OtherActor :type Actor%20Object%20Reference))
  ;[1 1 1] OnCollisionEvent
  (if (== (Utilities|GetClass OtherActor) "/Game/Imported/--Gamestarter--/FPS/Blueprints/PlayerProjectile_FPS.PlayerProjectile_FPS_C")
    (Actor|DestroyActor OtherActor)
    (Actor|DestroyActor)))

(event EventTick
  (params (DeltaSeconds :type Float%20%28single-precision%29))
  (bind _returnvalue (Transformation|GetActorTransform))
  (bind (_location _rotation _scale) (Math|Transform|BreakTransform _returnvalue))
  (AI|Navigation|SimpleMovetoActor (Pawn|GetController) (Game|GetPlayerCharacter 0))
  ;[1 1 1] Shoot Projectile After Random Time Has Passed
  (bind _output_get (Variables|Default|SetShootTimer (- (Variables|Default|GetShootTimer) DeltaSeconds)))
  (if (<= _output_get 0.0)
    (Game|SpawnActorfromClass "/Game/Imported/--Gamestarter--/FPS/Blueprints/EnemyProjectile_FPS.EnemyProjectile_FPS_C" (Math|Transform|MakeTransform (+ _location (* (Transformation|GetActorForwardVector) 2e+01)) _rotation _scale) "Undefined" 0 0)
    (Variables|Default|SetShootTimer (Math|Random|RandomFloatinRange 0.5 2.0))))

(fn ConstructionScript)