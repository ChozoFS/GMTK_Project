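; Enemy projectile actor that flies forward and damages the player character.
; On BeginPlay it sets the physics linear velocity of Sphere1 along the root's forward vector, scaled by BulletSpeed, and destroys itself after a fixed delay.
; A Sphere1 overlap with BP_PlayerCharacter applies fixed damage without destroying the projectile.
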(event OnComponentBeginOverlap(Sphere1)
  (params (OverlappedComponent :type Primitive%20Component%20Object%20Reference) (OtherActor :type Actor%20Object%20Reference) (OtherComp :type Primitive%20Component%20Object%20Reference) (OtherBodyIndex :type Integer) (bFromSweep :type Boolean) (SweepResult :type Hit%20Result%20Structure%20%28by%20ref%29))
  (bind _asbp_player_character (Utilities|Casting|CastToBP_PlayerCharacter OtherActor))
  (Game|Damage|ApplyDamage _asbp_player_character 1.0 0 0))

(event EventBeginPlay
  (Physics|SetPhysicsLinearVelocity (Variables|Default|GetSphere1) (* (* (Math|Vector|GetForwardVector (Variables|Default|GetDefaultSceneRoot)) (Variables|Default|GetBulletSpeed)) 1e+02) false "None")
  (Utilities|FlowControl|Delay 5.0)
  (Actor|DestroyActor))

(fn ConstructionScript)