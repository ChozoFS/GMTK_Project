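; BP_EnemyStrafe is an enemy that chases the player and fires projectiles at a fixed interval.
; Tick issues a simple move toward the player character and counts down a shoot timer, spawning BP_EnemyProjectile just ahead along its forward vector before resetting.
; Overlapping a BP_PlayerProjectile destroys both the projectile and the enemy.
; Despite the name, it has no strafing logic; a location-based move and a random-float node are left unused.
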(event EventBeginPlay
  ;[1 1 1] Shoot Projectile After Timer Has Passed
  (Variables|Default|SetShootTimer (Variables|Default|GetShootTimerSet)))

(event Collision|EventActorBeginOverlap
  (params (OtherActor :type Actor%20Object%20Reference))
  ;[1 1 1] OnCollisionEvent
  (if (== (Utilities|GetClass OtherActor) "/Game/Blueprints/BP_PlayerProjectile.BP_PlayerProjectile_C")
    (Actor|DestroyActor OtherActor)
    (Actor|DestroyActor)))

(event EventTick
  (params (DeltaSeconds :type Float%20%28single-precision%29))
  (bind _returnvalue (Transformation|GetActorTransform))
  (bind (_location _rotation _scale) (Math|Transform|BreakTransform _returnvalue))
  (AI|Navigation|SimpleMovetoActor (Pawn|GetController) (Game|GetPlayerCharacter 0))
  ;[1 1 1] Shoot Projectile After Timer Has Passed
  (bind _output_get (Variables|Default|SetShootTimer (- (Variables|Default|GetShootTimer) DeltaSeconds)))
  (if (<= _output_get 0.0)
    (Game|SpawnActorfromClass "/Game/Enemies/--Gamestarter--/FPS/Blueprints/BP_EnemyProjectile.BP_EnemyProjectile_C" (Math|Transform|MakeTransform (+ _location (* (Transformation|GetActorForwardVector) 2e+01)) _rotation _scale) "Undefined" 0 0)
    (Variables|Default|SetShootTimer (Variables|Default|GetShootTimerSet))))

(fn ConstructionScript)