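; BP_EnemyBase is a base enemy for an FPS that chases the player and fires projectiles.
; A looping timer set on BeginPlay spawns BP_EnemyProjectile just ahead of the enemy along its forward vector.
; Tick issues a simple AI move toward the player character every frame.
; Overlapping a BP_PlayerProjectile destroys both it and the enemy; disconnected nodes remain from an older Tick-based shoot countdown.
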(event Custom|Shoot
  (bind _returnvalue (Transformation|GetActorTransform))
  (bind (_location _rotation _scale) (Math|Transform|BreakTransform _returnvalue))
  ;[1 1 1] Shoots Based on Timer
  (Game|SpawnActorfromClass "/Game/Enemies/--Gamestarter--/FPS/Blueprints/BP_EnemyProjectile.BP_EnemyProjectile_C" (Math|Transform|MakeTransform (+ _location (* (Transformation|GetActorForwardVector) 2e+01)) _rotation _scale) "Undefined" 0 0))

(event EventBeginPlay
  ;[1 1 1] How often the enemies shoot
  (Utilities|Time|SetTimerbyEvent (delegate Custom|Shoot) (Variables|Default|GetShootTimer) true))

(event Collision|EventActorBeginOverlap
  (params (OtherActor :type Actor%20Object%20Reference))
  ;[1 1 1] OnCollisionEvent
  (Utilities|IsValid OtherActor
    (:Is%20Valid
      (if (== (Utilities|GetClass OtherActor) "/Game/Blueprints/BP_PlayerProjectile.BP_PlayerProjectile_C")
        (Actor|DestroyActor OtherActor)
        (Actor|DestroyActor)))))

(event EventTick
  (params (DeltaSeconds :type Float%20%28single-precision%29))
  ;[1 1 1] Moves the Actor towards the Player Character every frame.
  (AI|Navigation|SimpleMovetoActor (Pawn|GetController) (Game|GetPlayerCharacter 0)))

(fn ConstructionScript)