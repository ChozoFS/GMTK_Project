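; FPS enemy pawn that chases the player, fires projectiles and awards score when shot.
; Each tick it moves toward the player character with SimpleMoveToActor and counts down a randomized timer, spawning an EnemyProjectile_FPS just ahead of itself when it expires.
; Overlapping a PlayerProjectile_FPS destroys both actors and adds points through the Gamestarter_Blueprint found at BeginPlay.
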(event EventBeginPlay
  (bind _outactors (Actor|GetAllActorsOfClass "/Game/ImportedThings/--Gamestarter--/Gamestarter_Blueprint.Gamestarter_Blueprint_C"))
  (Variables|Default|SetGamestarter_Blueprint (Utilities|Array|Get(acopy) _outactors))
  ;[1 1 1] Shoot Projectile After Random Time Has Passed
  (Variables|Default|SetShootTimer (Math|Random|RandomFloatinRange 0.5 2.0)))

(event Collision|EventActorBeginOverlap
  (params (OtherActor :type Actor%20Object%20Reference))
  ;[1 1 1] OnCollisionEvent
  (if (== (Utilities|GetClass OtherActor) "/Game/ImportedThings/--Gamestarter--/FPS/Blueprints/PlayerProjectile_FPS.PlayerProjectile_FPS_C")
    (Actor|DestroyActor OtherActor)
    (Default|CallOnAddScore (Variables|Default|GetGamestarter_Blueprint) 100)
    (Actor|DestroyActor)))

(event EventTick
  (params (DeltaSeconds :type Float%20%28single-precision%29))
  (bind _returnvalue (Transformation|GetActorTransform))
  (bind (_location _rotation _scale) (Math|Transform|BreakTransform _returnvalue))
  (AI|Navigation|SimpleMovetoActor (Pawn|GetController) (Game|GetPlayerCharacter 0))
  ;[1 1 1] Shoot Projectile After Random Time Has Passed
  (bind _output_get (Variables|Default|SetShootTimer (- (Variables|Default|GetShootTimer) DeltaSeconds)))
  (if (<= _output_get 0.0)
    (Game|SpawnActorfromClass "/Game/ImportedThings/--Gamestarter--/FPS/Blueprints/EnemyProjectile_FPS.EnemyProjectile_FPS_C" (Math|Transform|MakeTransform (+ _location (* (Transformation|GetActorForwardVector) 2e+01)) _rotation _scale) "Undefined" 0 0)
    (Variables|Default|SetShootTimer (Math|Random|RandomFloatinRange 0.5 2.0))))

(fn ConstructionScript)