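; Soccer ball actor that detects when it enters a goal and reports the score to the Gamestarter system.
; On BeginPlay it finds and caches the first Gamestarter_Blueprint actor in the level.
; When it overlaps an actor whose class is exactly GoalTrigger, it passes that trigger's WhichTeamPoint to CallOnSoccerGoal on the cached Gamestarter.
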(event EventBeginPlay
  (bind _outactors (Actor|GetAllActorsOfClass "/Game/ImportedThings/--Gamestarter--/Gamestarter_Blueprint.Gamestarter_Blueprint_C"))
  (Variables|Default|SetGameStarter%20Blueprint (Utilities|Array|Get(acopy) _outactors)))

(event Collision|EventActorBeginOverlap
  (params (OtherActor :type Actor%20Object%20Reference))
  (if (== (Utilities|GetClass OtherActor) "/Game/ImportedThings/--Gamestarter--/Soccer/Blueprints/GoalTrigger.GoalTrigger_C")
    (bind _asgoal_trigger (Utilities|Casting|CastToGoalTrigger OtherActor))
    (Default|CallOnSoccerGoal (Variables|Default|GetGameStarter%20Blueprint) (Variables|/Game/ImportedThings/--Gamestarter--/Soccer/Blueprints/GoalTrigger.GoalTrigger_C|GetWhichTeamPoint _asgoal_trigger))))

(event EventTick
  (params (DeltaSeconds :type Float%20%28single-precision%29)))

(fn ConstructionScript)