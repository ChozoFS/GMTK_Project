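; Follow camera actor for a platformer that trails a PlayerToFollow actor along the X axis.
; Each Tick, if the player is valid and outside a small dead zone, it moves toward the player at a speed proportional to their X distance, giving a frame-time-scaled eased follow.
; Y and Z stay fixed, so the camera never tracks vertical or depth movement.
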(event EventBeginPlay)

(event Collision|EventActorBeginOverlap
  (params (OtherActor :type Actor%20Object%20Reference)))

(event EventTick
  (params (DeltaSeconds :type Float%20%28single-precision%29))
  (bind _returnvalue (Transformation|GetActorLocation))
  (bind _returnvalue_2 (Transformation|GetActorLocation))
  (bind _playertofollow (Variables|Default|GetPlayerToFollow))
  (bind (_x _y _z) (Math|Vector|BreakVector _returnvalue))
  (bind _returnvalue_3 (Transformation|GetActorLocation _playertofollow))
  (bind (_x_2 _y_2 _z_2) (Math|Vector|BreakVector _returnvalue_2))
  (bind _x_3 (Math|Vector|BreakVector _returnvalue_3))
  (Utilities|IsValid _playertofollow
    (:Is%20Valid
      (if (> _x_3 (+ _x 5.0))
        (Transformation|SetActorLocation (Math|Vector|MakeVector (+ _x (* DeltaSeconds (* (Math|Float|Absolute(Float) (- _x_3 _x)) 4.0))) _y _z) false false)
        (elif (< _x_3 (- _x 5.0))
          (Transformation|SetActorLocation (Math|Vector|MakeVector (- _x_2 (* DeltaSeconds (* (Math|Float|Absolute(Float) (- _x_3 _x_2)) 4.0))) _y_2 _z_2) false false))))))

(fn ConstructionScript)